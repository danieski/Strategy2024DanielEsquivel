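; BP_Bullet is a projectile actor that travels toward one assigned target and damages it on contact.
; On BeginPlay it adds a BPC move-to-target component, passing in the target and bullet speed.
; Its sphere overlap ignores every actor except that target, then applies damage credited to the first player controller and destroys the bullet.
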(event OnComponentBeginOverlap(Sphere)
  (params (OverlappedComponent :type Primitive%20Component%20Object%20Reference) (OtherActor :type Actor%20Object%20Reference) (OtherComp :type Primitive%20Component%20Object%20Reference) (OtherBodyIndex :type Integer) (bFromSweep :type Boolean) (SweepResult :type Hit%20Result%20Structure%20%28by%20ref%29))
  (bind _mtarget (Variables|Default|GetmTarget))
  (if (== OtherActor _mtarget)
    (Game|Damage|ApplyDamage _mtarget (Variables|Default|GetmDamage) (Game|GetPlayerController 0) self)
    (Actor|DestroyActor)))

(event EventBeginPlay
  (AddComponent|AddBPCMovetoTarget (Variables|Default|GetmTarget) (Variables|Default|GetmBulletSpeed)))

(fn ConstructionScript)