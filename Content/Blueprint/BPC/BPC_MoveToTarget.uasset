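; BPC_MoveToTarget is a component that makes its owning actor home in on a target actor.
; Each tick it moves the owner straight along the normalized direction to MTarget at MSpeed, scaled by delta time, and rotates it to face the target.
; It sets the transform directly, has no arrival check, and destroys the owner once MTarget is no longer valid.
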(event EventTick
  (params (DeltaSeconds :type Float%20%28single-precision%29))
  (bind _returnvalue (Components|GetOwner))
  (bind _mtarget (Variables|Default|GetmTarget))
  (bind _returnvalue_2 (Transformation|GetActorLocation _mtarget))
  (bind _returnvalue_3 (Transformation|GetActorLocation _returnvalue))
  (Variables|Default|GetmTarget
    (:then
      (Transformation|SetActorLocationAndRotation (Components|GetOwner) (+ (* (* DeltaSeconds (Variables|Default|GetmSpeed)) (Math|Vector|Normalize (- _returnvalue_2 _returnvalue_3))) _returnvalue_3) (Math|Rotator|FindLookatRotation _returnvalue_3 _returnvalue_2)))
    (:else
      (Actor|DestroyActor (Components|GetOwner)))))