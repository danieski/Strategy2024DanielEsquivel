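; BP_Turret is a turret actor that automatically shoots BP_Bullet projectiles at a single BP_Enemy target within its radius.
; Construction loads damage, shoot speed and bullet speed from DT_Turrets by turret name.
; ShootRadius overlaps set or clear the target, acquiring only on overlap begin when none is valid.
; A looping fire-rate timer spawns bullets carrying target and stats, and starts a timeline turn toward the enemy with zero pitch.
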(event OnComponentEndOverlap(ShootRadius)
  (params (OverlappedComponent :type Primitive%20Component%20Object%20Reference) (OtherActor :type Actor%20Object%20Reference) (OtherComp :type Primitive%20Component%20Object%20Reference) (OtherBodyIndex :type Integer))
  (if (== (Variables|Default|GetmTarget) OtherActor)
    (Variables|Default|SetmTarget 0)))

(event OnComponentBeginOverlap(ShootRadius)
  (params (OverlappedComponent :type Primitive%20Component%20Object%20Reference) (OtherActor :type Actor%20Object%20Reference) (OtherComp :type Primitive%20Component%20Object%20Reference) (OtherBodyIndex :type Integer) (bFromSweep :type Boolean) (SweepResult :type Hit%20Result%20Structure%20%28by%20ref%29))
  (Variables|Default|GetmTarget
    (:then)
    (:else
      (Utilities|Casting|CastToBP_Enemy OtherActor)
      (Variables|Default|SetmTarget OtherActor))))

(event Custom|ShootTick
  (Variables|Default|GetmTarget
    (:then
      (CallFunction|RotatetoTarget)
      (Game|SpawnActorfromClass "/Game/Blueprint/BP_Bullet.BP_Bullet_C" (Math|Transform|MakeTransform (Transformation|GetWorldLocation (Variables|Default|GetShootPoint)) "0, 0, 0" "1.000000,1.000000,1.000000") "Undefined" "MultiplyWithRoot" self (Variables|Default|GetmBulletSpeed) (Variables|Default|GetmBulletDamage) (Variables|Default|GetmTarget) 1.0 0))
    (:else)))

(event Custom|RotateToTarget
  (bind _returnvalue (Transformation|GetActorLocation))
  (bind _mtarget (Variables|Default|GetmTarget))
  (bind _returnvalue_2 (Transformation|GetActorLocation _mtarget))
  (bind _returnvalue_3 (Math|Rotator|FindLookatRotation _returnvalue _returnvalue_2))
  (Variables|Default|SetmAuxrot (Transformation|GetActorRotation))
  (Components|Timeline|SetPlayRate (Variables|Default|GetLepRotation) (Variables|Default|GetmShootSpeed))
  (bind _time (Timeline|LepRotation Play)
    (:Update
      (Variables|Default|GetmTarget
        (:then
          (Transformation|SetActorRotation (Math|Rotator|Lerp(Rotator) (Variables|Default|GetmAuxrot) (Math|Rotator|MakeRotator (.roll _returnvalue_3) 0.0 (.yaw _returnvalue_3)) _time)))
        (:else
          (Timeline|LepRotation Stop))))))

(event EventBeginPlay
  (Utilities|Time|SetTimerbyEvent (delegate Custom|ShootTick) (CallFunction|FGetShootSpeed) true))

(fn ConstructionScript
  (bind _returnvalue (Utilities|GetDataTableRow "/Game/Blueprint/DT_Turrets.DT_Turrets" (Variables|Default|GetTURRET%20NAME))
    (:then
      (Utilities|FlowControl|Sequence
        (:then_0
          (Variables|Default|SetmBulletDamage (.mDamage (Utilities|Struct|BreaksTurretInfo _returnvalue))))
        (:then_1
          (Variables|Default|SetmShootSpeed (.mShootSpeed (Utilities|Struct|BreaksTurretInfo _returnvalue))))
        (:then_2
          (Variables|Default|SetmBulletSpeed (.mBulletSpeed (Utilities|Struct|BreaksTurretInfo _returnvalue))))))))

(fn FGetShootSpeed
  (return (/ 1.0 (Variables|Default|GetmShootSpeed))))