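; Enemy pawn Blueprint that walks a sequence of waypoints and destroys itself after reaching the last one.
; On BeginPlay it spawns its default controller, then AI MoveTo targets each waypoint offset by the stored spawner location.
; Each successful move increments the index and repeats; a failed move has no handling.
; Incoming damage only prints a debug message with the amount, without affecting health.
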(event Custom|GoToNextWaypoint
  (AI|AIMoveTo self (+ (Utilities|Array|Get(acopy) (Variables|Default|GetmWaypoints) (Variables|Default|GetmCurrentWaypoint)) (Variables|Default|GetmSpaownerLocation)) 0 5.0 false
    (:OnSuccess
      (bind _result (Math|Integer|IncrementInt (Variables|Default|GetmCurrentWaypoint))
        (:%20%20
          (if (Utilities|Array|IsValidIndex (Variables|Default|GetmWaypoints) _result)
            (CallFunction|GotoNextWaypoint)
            (else
              (Actor|DestroyActor))))))))

(event EventBeginPlay
  (Utilities|FlowControl|Sequence
    (:then_0
      (Pawn|SpawnDefaultController))
    (:then_1
      (CallFunction|GotoNextWaypoint))))

(event Game|Damage|EventAnyDamage
  (params (Damage :type Float%20%28single-precision%29) (DamageType :type Damage%20Type%20Object%20Reference) (InstigatedBy :type Controller%20Object%20Reference) (DamageCauser :type Actor%20Object%20Reference))
  (Development|PrintString (Utilities|String|Append "Me putearon" (Utilities|String|ToString(Float) Damage))))

(fn ConstructionScript)