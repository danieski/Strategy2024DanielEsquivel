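; Enemy spawner actor that spawns a BP_Enemy at its own transform every few seconds, indefinitely from BeginPlay.
; Each enemy receives the spawner's local-space waypoint array and world location at spawn.
; FDrawLine previews the route with long-lived debug lines from the spawner through each transformed waypoint.
; It runs at BeginPlay and in the construction script, which first flushes persistent debug lines to refresh the preview.
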(event EventBeginPlay
  (Utilities|FlowControl|Sequence
    (:then_0
      (CallFunction|FDrawLine))
    (:then_1
      (Utilities|FlowControl|Delay 5.0 :!label _label)
      (Game|SpawnActorfromClass "/Game/Blueprint/Enemies/BP_Enemy.BP_Enemy_C" (Transformation|GetActorTransform) "AlwaysSpawn" "MultiplyWithRoot" 0 (Variables|Default|GetmWayPoints) (Transformation|GetActorLocation) 0)
      (goto _label))))

(fn ConstructionScript
  (Rendering|Debug|FlushPersistentDebugLines)
  (CallFunction|FDrawLine))

(fn FDrawLine
  (bind _returnvalue (Transformation|GetActorTransform))
  (if (Utilities|Array|IsNotEmpty (Variables|Default|GetmWayPoints))
    (for (_array_element _array_index) (Variables|Default|GetmWayPoints)
      (if (< _array_index 1)
        (Rendering|Debug|DrawDebugLine :LineStart (Transformation|GetActorLocation) :LineEnd (Math|Transform|TransformLocation _returnvalue _array_element) :Duration 990999.0 :Thickness 1e+01)
        (else
          (Rendering|Debug|DrawDebugLine :LineStart (Math|Transform|TransformLocation _returnvalue _array_element) :LineEnd (Math|Transform|TransformLocation _returnvalue (Utilities|Array|Get(acopy) (Variables|Default|GetmWayPoints) (- _array_index 1))) :Duration 9999999.0 :Thickness 1e+01))))))