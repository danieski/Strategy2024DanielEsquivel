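; Player controller that lets the player place a selected turret in the world with the mouse and open the shop.
; On BeginPlay it adds the Enhanced Input mapping context, hides and locks the cursor in Game and UI mode, and caches BP_HUD.
; Left click spawns the selected turret's prefab, if valid, at a WorldStatic line trace from the deprojected mouse position.
; Right click opens the shop through the HUD.
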(event Input|EnhancedActionEvents|EnhancedInputActionIA_LeftClick
  (params (ActionValue :type Boolean) (ElapsedSeconds :type Float%20%28double-precision%29) (TriggeredSeconds :type Float%20%28double-precision%29) (InputAction :type Input%20Action%20Object%20Reference :default "/Game/Inputs/IA_LeftClick.IA_LeftClick"))
  (bind (_worldlocation _worlddirection) (Game|Player|ConvertMouseLocationToWorldSpace))
  (bind _mprefab (Utilities|HasTurretSelected)
    (:true
      (bind _outhit (Collision|LineTraceForObjects _worldlocation (+ _worldlocation (* _worlddirection 3500)) (Utilities|Array|MakeArray "ObjectTypeQuery1") false 0 "ForDuration"))
      (Game|SpawnActorfromClass _mprefab (Math|Transform|MakeTransform (.ImpactPoint (Collision|BreakHitResult _outhit)) "0, 0, 0" "1.000000,1.000000,1.000000") "Undefined" "MultiplyWithRoot" 0 0))))

(event Input|EnhancedActionEvents|EnhancedInputActionIA_RightClick
  (params (ActionValue :type Boolean) (ElapsedSeconds :type Float%20%28double-precision%29) (TriggeredSeconds :type Float%20%28double-precision%29) (InputAction :type Input%20Action%20Object%20Reference :default "/Game/Inputs/IA_RightClick.IA_RightClick"))
  (:Started
    (Default|OpenShop (Variables|Default|GetAs%20BP%20HUD))))

(event EventBeginPlay
  (Utilities|FlowControl|Sequence
    (:then_0
      (Input|AddMappingContext (PlayerController|LocalPlayerSubsystems|GetEnhancedInputLocalPlayerSubsystem) "/Game/Inputs/ICM_Base.ICM_Base" 0 "(bIgnoreAllPressedKeysUntilRelease=True,bForceImmediately=False,bNotifyUserSettings=False)"))
    (:then_1
      (Variables|Default|SetbShowMouseCursor false)
      (Input|SetInputModeGameandUI self 0 "LockAlways" true false))
    (:then_2
      (bind _asbp_hud (Utilities|Casting|CastToBP_HUD (HUD|GetHUD)))
      (Variables|Default|SetAs%20BP%20HUD _asbp_hud))))

(fn ConstructionScript)